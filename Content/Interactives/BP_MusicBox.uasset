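; BP_MusicBox is an interactive music box that accepts a cylinder carried by the player.
; The Cylinder component starts hidden, and looking at the box adds the player's InteractRef widget to the viewport until a cylinder is placed.
; Interacting while holding a cylinder clears the player's HasCylinder flag, sets PlacedCylinder and reveals the component.
; No audio playback is implemented here.
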(event EventLookat
  (params (PlayerChar :type BP%20Third%20Person%20Character%20Object%20Reference))
  (if (not (Variables|Default|GetPlacedCylinder?))
    (UserInterface|Viewport|AddtoViewport (Variables|/Game/ThirdPerson/Blueprints/BP_ThirdPersonCharacter.BP_ThirdPersonCharacter_C|GetInteractRef PlayerChar) 0)))

(event EventInteractwith
  (params (PlayerChar :type BP%20Third%20Person%20Character%20Object%20Reference))
  (if (Variables|/Game/ThirdPerson/Blueprints/BP_ThirdPersonCharacter.BP_ThirdPersonCharacter_C|GetHasCylinder? PlayerChar)
    (Variables|/Game/ThirdPerson/Blueprints/BP_ThirdPersonCharacter.BP_ThirdPersonCharacter_C|SetHasCylinder? PlayerChar false)
    (Variables|Default|SetPlacedCylinder? true)
    (if (Variables|Default|GetPlacedCylinder?)
      (Rendering|SetVisibility (Variables|Default|GetCylinder) true false))))

(event EventBeginPlay
  (Rendering|SetVisibility (Variables|Default|GetCylinder) false false))

(fn ConstructionScript)