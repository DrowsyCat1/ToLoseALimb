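; BP_Box is an interactive box actor that the player can move once.
; On Interactwith it jumps to a preset NewLocation without sweeping and sets HasMoved so later interactions do nothing.
; While it has not moved, Lookat adds the looking player's InteractRef widget to the viewport as a prompt.
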(event EventInteractwith
  (params (PlayerChar :type BP%20Third%20Person%20Character%20Object%20Reference))
  (if (not (Variables|Default|GetHasMoved?))
    (Transformation|SetActorLocation (Variables|Default|GetNewLocation) false false)
    (Variables|Default|SetHasMoved? true)))

(event EventLookat
  (params (PlayerChar :type BP%20Third%20Person%20Character%20Object%20Reference))
  (if (not (Variables|Default|GetHasMoved?))
    (UserInterface|Viewport|AddtoViewport (Variables|/Game/ThirdPerson/Blueprints/BP_ThirdPersonCharacter.BP_ThirdPersonCharacter_C|GetInteractRef PlayerChar) 0)))

(fn ConstructionScript
  (|CallParentFunction))