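; BP_PullPlank is a one-shot interactable plank that plays a level sequence when the player interacts with it.
; On first interaction it starts the sequence, teleports the player to a hard-coded location, plays a metal crash sound at world origin and destroys itself.
; A HasMoved flag guards both the interaction and the look-at event, which adds the player's interact prompt widget to the viewport.
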(event EventInteractwith
  (params (PlayerChar :type BP%20Third%20Person%20Character%20Object%20Reference))
  (if (not (Variables|Default|GetHasMoved?))
    (bind _outactor (Sequencer|Player|CreateLevelSequencePlayer (Variables|Default|GetLevel%20Sequence)))
    (Sequencer|Player|Play (Variables|/Script/LevelSequence.LevelSequenceActor|GetSequencePlayer _outactor) :!class /Script/MovieScene.MovieSceneSequencePlayer)
    (Variables|Default|SetHasMoved? true)
    (Transformation|SetActorLocationAndRotation (Game|GetPlayerCharacter 0) "-1250.000000,1809.000000,90.000000")
    (Audio|PlaySoundatLocation "/Game/sounds/light-metal-crash-6765_Cue.light-metal-crash-6765_Cue" "0, 0, 0" "0, 0, 0" 1.0 1.0 0.0 0 0 0 0)
    (Actor|DestroyActor)))

(event EventLookat
  (params (PlayerChar :type BP%20Third%20Person%20Character%20Object%20Reference))
  (if (not (Variables|Default|GetHasMoved?))
    (UserInterface|Viewport|AddtoViewport (Variables|/Game/ThirdPerson/Blueprints/BP_ThirdPersonCharacter.BP_ThirdPersonCharacter_C|GetInteractRef PlayerChar) 0)))

(fn ConstructionScript
  (|CallParentFunction))